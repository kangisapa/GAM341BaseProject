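; A basic player Character Blueprint that handles movement, look, crouch, run and jump input.
; Axis inputs drive movement along the actor's forward and right vectors and rotate the controller's yaw and pitch.
; Hold-to-crouch and hold-to-run toggle crouching and swap walk speed between walk and run values.
; Jumping plays a sound at the capsule and sets max hold time from the public InAirTime variable, stopping on release.
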(event Input|ActionEvents|InputActionJump
  (params (Key :type Key%20Structure :default "None"))
  ;[1 1 1] Jump Controls. Variable inAirTime is a public variable that can be changed in game.
  (:Pressed
    (Variables|Default|SetJumpMaxHoldTime (Variables|Default|GetinAirTime))
    (Audio|PlaySoundatLocation "/Game/Audio/PlayerJump.PlayerJump" (Transformation|GetWorldLocation (Variables|Collision|GetCapsuleComponent)) "0, 0, 0" 1.0 1.0 0.0 0 0 0)
    (Character|Jump))
  (:Released
    (Character|StopJumping)))

(event Input|ActionEvents|InputActionRun
  (params (Key :type Key%20Structure :default "None"))
  (bind _charactermovement (Variables|Character|GetCharacterMovement))
  ;[1 1 1] Run and Walk controls
  (:Pressed
    (Variables|/Script/Engine.CharacterMovementComponent|SetMaxWalkSpeed _charactermovement (Variables|Default|GetMaxRunSpeed)))
  (:Released
    (Variables|/Script/Engine.CharacterMovementComponent|SetMaxWalkSpeed _charactermovement (Variables|Default|GetMaxWalkSpeed))))

(event Input|ActionEvents|InputActionCrouch
  (params (Key :type Key%20Structure :default "None"))
  ;[1 1 1] Crouch Controls
  (:Pressed
    (Character|Crouch))
  (:Released
    (Character|UnCrouch)))

(event Input|AxisEvents|InputAxisForward/Backward
  (params (AxisValue :type Float%20%28single-precision%29))
  ;[0.4328 0.5816 1] Player Movement Forward/Back/Left/Right
  (Pawn|Input|AddMovementInput (Transformation|GetActorForwardVector) AxisValue false))

(event Input|AxisEvents|InputAxisRight/Left
  (params (AxisValue :type Float%20%28single-precision%29))
  ;[0.4328 0.5816 1] Player Movement Forward/Back/Left/Right
  (Pawn|Input|AddMovementInput (Transformation|GetActorRightVector) AxisValue false))

(event Input|AxisEvents|InputAxisLook_Left/Right
  (params (AxisValue :type Float%20%28single-precision%29))
  ;[0.4769 0.5228 1] Player Look Up/Down/Left/Right
  (Pawn|Input|AddControllerYawInput AxisValue))

(event Input|AxisEvents|InputAxisLook_Up/Down
  (params (AxisValue :type Float%20%28single-precision%29))
  ;[0.4769 0.5228 1] Player Look Up/Down/Left/Right
  (Pawn|Input|AddControllerPitchInput AxisValue))

(fn ConstructionScript)